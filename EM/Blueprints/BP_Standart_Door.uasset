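; BP_Standart_Door is a proximity door that swings open when the player character enters its CollisionEnter volume and closes when they leave.
; Overlap begin plays a timeline that drives the door body's relative yaw, and overlap end reverses it.
; Each update prints the angle and disables the body's collision at -50 degrees or below, restoring it otherwise.
; The CollisionExit overlap event is an empty stub.
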(event OnComponentBeginOverlap(CollisionEnter)
  (params (OtherActor :type Actor%20Object%20Reference) (OtherComp :type Primitive%20Component%20Object%20Reference) (OtherBodyIndex :type Integer) (bFromSweep :type Boolean) (SweepResult :type Hit%20Result%20Structure%20%28by%20ref%29))
  (bind _door_standart_movable_door_body (Variables|Default|Getdoor_standart_movable_door_body))
  (if (== (Game|GetPlayerCharacter 0) OtherActor)
    (bind _rotation (Timeline|Timeline_0 Play)
      (:Update
        (Development|PrintString (Utilities|String|ToString(Float) _rotation))
        (Transformation|SetRelativeRotation (Variables|Default|Getdoor_standart_movable_door_body) (Math|Rotator|MakeRotator 0.0 0.0 _rotation) false false)
        (if (<= _rotation -5e+01)
          (Collision|SetCollisionEnabled _door_standart_movable_door_body "NoCollision")
          (else
            (Collision|SetCollisionEnabled _door_standart_movable_door_body "QueryAndPhysics")))))))

(event OnComponentEndOverlap(CollisionEnter)
  (params (OtherActor :type Actor%20Object%20Reference) (OtherComp :type Primitive%20Component%20Object%20Reference) (OtherBodyIndex :type Integer))
  (bind _door_standart_movable_door_body (Variables|Default|Getdoor_standart_movable_door_body))
  (if (== (Game|GetPlayerCharacter 0) OtherActor)
    (bind _rotation (Timeline|Timeline_0 Reverse)
      (:Update
        (Development|PrintString (Utilities|String|ToString(Float) _rotation))
        (Transformation|SetRelativeRotation (Variables|Default|Getdoor_standart_movable_door_body) (Math|Rotator|MakeRotator 0.0 0.0 _rotation) false false)
        (if (<= _rotation -5e+01)
          (Collision|SetCollisionEnabled _door_standart_movable_door_body "NoCollision")
          (else
            (Collision|SetCollisionEnabled _door_standart_movable_door_body "QueryAndPhysics")))))))

(event OnComponentBeginOverlap(CollisionExit)
  (params (OtherActor :type Actor%20Object%20Reference) (OtherComp :type Primitive%20Component%20Object%20Reference) (OtherBodyIndex :type Integer) (bFromSweep :type Boolean) (SweepResult :type Hit%20Result%20Structure%20%28by%20ref%29)))

(event EventBeginPlay)

(event Collision|EventActorBeginOverlap
  (params (OtherActor :type Actor%20Object%20Reference)))

(event EventTick
  (params (DeltaSeconds :type Float%20%28single-precision%29)))

(fn ConstructionScript)