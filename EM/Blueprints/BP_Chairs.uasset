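; BP_Chairs manages rows of seating, spawning Basic or Better chair actors according to ChairName.
; Target actors passed in set chairs per row and base positions, with each further row offset along Y.
; Adding or removing a row waits briefly, then destroys and respawns the current type's chairs; changing type only destroys them.
; Positioning indexes BPBasicChairsArray, though live spawns fill the Lucca and Teatro arrays; several older graph chains are disconnected.
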(event Custom|ArrayLoopForLocation
  (for _index (range 0 (* (Variables|Default|GetRows) (Variables|Default|GetChairsInRow)))
    (switch name (Variables|Default|GetChairName)
      (:BasicChair
        (bind _returnvalue (Game|SpawnActorfromClass 0 (Math|Conversions|ToTransform(Vector) (Variables|Default|GetCurrentTargetLocation)) "AdjustIfPossibleButDontSpawnIfColliding" 0 0))
        (bind _output_get (Variables|Default|SetBP_LuccaChair _returnvalue))
        (bind _returnvalue_2 (Utilities|Array|Add (Variables|Default|GetBP_LuccaChairArray) _output_get))
        (Variables|Default|SetCurrentMeshIndex _returnvalue_2))
      (:BetterChair
        (bind _returnvalue_3 (Game|SpawnActorfromClass 0 (Math|Conversions|ToTransform(Vector) (Variables|Default|GetCurrentTargetLocation)) "AdjustIfPossibleButDontSpawnIfColliding" 0 0))
        (bind _output_get_2 (Variables|Default|SetBP_TeatroChair _returnvalue_3))
        (bind _returnvalue_4 (Utilities|Array|Add (Variables|Default|GetBP_TeatroChairArray) _output_get_2))
        (Variables|Default|SetCurrentMeshIndex _returnvalue_4)))
    (Variables|Default|SetCurrentChairsInRow (+ (Variables|Default|GetCurrentChairsInRow) 1))
    (Variables|Default|SetIndex2ndLoop_Targets (+ (Variables|Default|GetIndex2ndLoop_Targets) 1))
    (if (> (Variables|Default|GetIndex2ndLoop_Targets) (Variables|Default|GetChairsInRow))
      (Variables|Default|SetIndex2ndLoop_Targets 0))
    (for _index_2 (range (Variables|Default|GetIndex2ndLoop_Targets) (Variables|Default|GetIndex2ndLoop_Targets))
      (Variables|Default|SetCurrentTargetIndexx _index_2)
      (if (>= (Variables|Default|GetCurrentChairsInRow) (Variables|Default|GetChairsInRow))
        (Variables|Default|SetCurrentChairsInRow -1)
        (Variables|Default|SetRowLocation (+ (Variables|Default|GetRowLocation) "0,150.000000, 0")))
      (Variables|Default|SetCurrentTargetLocation (- (Transformation|GetActorLocation (Utilities|Array|Get(acopy) (Variables|Default|GetTargets) (Variables|Default|GetCurrentTargetIndexx))) (Variables|Default|GetRowLocation)))
      (Rendering|SetActorHiddenInGame false)
      (Transformation|SetActorLocationAndRotation (Utilities|Array|Get(acopy) (Variables|Default|GetBP_BasicChairsArray) (Variables|Default|GetCurrentMeshIndex)) (- (Transformation|GetActorLocation (Utilities|Array|Get(acopy) (Variables|Default|GetTargets) (Variables|Default|GetCurrentTargetIndexx))) (Variables|Default|GetRowLocation)) (Transformation|GetActorRotation (Utilities|Array|Get(acopy) (Variables|Default|GetTargets) (Variables|Default|GetCurrentTargetIndexx))))))
  (Variables|Default|SetRowLocation "0, 0, 0")
  (Variables|Default|SetCurrentTargetLocation "0, 0, 0")
  (Variables|Default|SetCurrentChairsInRow 0)
  (Variables|Default|SetIndex2ndLoop_Targets 0))

(event Custom|SetHidden)

(event Custom|ChairMesh
  (params (01 :type Actor%20Object%20Reference) (02 :type Actor%20Object%20Reference))
  (Variables|Default|SetSpawnChair01 01)
  (Variables|Default|SetSpawnChair02 02))

(event Custom|MinusRow
  (Variables|Default|SetRows (- (Variables|Default|GetRows) 1))
  (Utilities|FlowControl|Delay 0.5)
  (Utilities|FlowControl|Sequence
    (:then_0
      (switch name (Variables|Default|GetChairName)
        (:BasicChair
          (for _array_element (Variables|Default|GetBP_LuccaChairArray)
            (Actor|DestroyActor _array_element)))
        (:BetterChair
          (for _array_element_2 (Variables|Default|GetBP_TeatroChairArray)
            (Actor|DestroyActor _array_element_2)))))
    (:then_1
      (for _index (range 0 (* (Variables|Default|GetRows) (Variables|Default|GetChairsInRow)))
        (switch name (Variables|Default|GetChairName)
          (:BasicChair
            (bind _returnvalue (Game|SpawnActorfromClass 0 (Math|Conversions|ToTransform(Vector) (Variables|Default|GetCurrentTargetLocation)) "AdjustIfPossibleButDontSpawnIfColliding" 0 0))
            (bind _output_get (Variables|Default|SetBP_LuccaChair _returnvalue))
            (bind _returnvalue_2 (Utilities|Array|Add (Variables|Default|GetBP_LuccaChairArray) _output_get))
            (Variables|Default|SetCurrentMeshIndex _returnvalue_2))
          (:BetterChair
            (bind _returnvalue_3 (Game|SpawnActorfromClass 0 (Math|Conversions|ToTransform(Vector) (Variables|Default|GetCurrentTargetLocation)) "AdjustIfPossibleButDontSpawnIfColliding" 0 0))
            (bind _output_get_2 (Variables|Default|SetBP_TeatroChair _returnvalue_3))
            (bind _returnvalue_4 (Utilities|Array|Add (Variables|Default|GetBP_TeatroChairArray) _output_get_2))
            (Variables|Default|SetCurrentMeshIndex _returnvalue_4)))
        (Variables|Default|SetCurrentChairsInRow (+ (Variables|Default|GetCurrentChairsInRow) 1))
        (Variables|Default|SetIndex2ndLoop_Targets (+ (Variables|Default|GetIndex2ndLoop_Targets) 1))
        (if (> (Variables|Default|GetIndex2ndLoop_Targets) (Variables|Default|GetChairsInRow))
          (Variables|Default|SetIndex2ndLoop_Targets 0))
        (for _index_2 (range (Variables|Default|GetIndex2ndLoop_Targets) (Variables|Default|GetIndex2ndLoop_Targets))
          (Variables|Default|SetCurrentTargetIndexx _index_2)
          (if (>= (Variables|Default|GetCurrentChairsInRow) (Variables|Default|GetChairsInRow))
            (Variables|Default|SetCurrentChairsInRow -1)
            (Variables|Default|SetRowLocation (+ (Variables|Default|GetRowLocation) "0,150.000000, 0")))
          (Variables|Default|SetCurrentTargetLocation (- (Transformation|GetActorLocation (Utilities|Array|Get(acopy) (Variables|Default|GetTargets) (Variables|Default|GetCurrentTargetIndexx))) (Variables|Default|GetRowLocation)))
          (Rendering|SetActorHiddenInGame false)
          (Transformation|SetActorLocationAndRotation (Utilities|Array|Get(acopy) (Variables|Default|GetBP_BasicChairsArray) (Variables|Default|GetCurrentMeshIndex)) (- (Transformation|GetActorLocation (Utilities|Array|Get(acopy) (Variables|Default|GetTargets) (Variables|Default|GetCurrentTargetIndexx))) (Variables|Default|GetRowLocation)) (Transformation|GetActorRotation (Utilities|Array|Get(acopy) (Variables|Default|GetTargets) (Variables|Default|GetCurrentTargetIndexx))))))
      (Variables|Default|SetRowLocation "0, 0, 0")
      (Variables|Default|SetCurrentTargetLocation "0, 0, 0")
      (Variables|Default|SetCurrentChairsInRow 0)
      (Variables|Default|SetIndex2ndLoop_Targets 0))))

(event Custom|ChairsMeshes
  (params (01 :type Array%20of%20Actor%20Object%20References)))

(event Custom|ChairsTargets
  (params (01 :type Array%20of%20Actor%20Object%20References))
  (bind _output_get (Variables|Default|SetTargets 01))
  (Variables|Default|SetChairsInRow (Utilities|Array|Length _output_get)))

(event Custom|ChairNameE
  (params (NewParam :type Name :default "None"))
  (CallFunction|DestroyActors)
  (Variables|Default|SetChairName NewParam))

(event Custom|DestroyActors
  (switch name (Variables|Default|GetChairName)
    (:BasicChair
      (for _array_element (Variables|Default|GetBP_LuccaChairArray)
        (Actor|DestroyActor _array_element)))
    (:BetterChair
      (for _array_element_2 (Variables|Default|GetBP_TeatroChairArray)
        (Actor|DestroyActor _array_element_2)))))

(event Custom|NumberRows
  (Variables|Default|SetRows (+ (Variables|Default|GetRows) 1))
  (Utilities|FlowControl|Delay 0.5)
  (Utilities|FlowControl|Sequence
    (:then_0
      (switch name (Variables|Default|GetChairName)
        (:BasicChair
          (for _array_element (Variables|Default|GetBP_LuccaChairArray)
            (Actor|DestroyActor _array_element)))
        (:BetterChair
          (for _array_element_2 (Variables|Default|GetBP_TeatroChairArray)
            (Actor|DestroyActor _array_element_2)))))
    (:then_1
      (for _index (range 0 (* (Variables|Default|GetRows) (Variables|Default|GetChairsInRow)))
        (switch name (Variables|Default|GetChairName)
          (:BasicChair
            (bind _returnvalue (Game|SpawnActorfromClass 0 (Math|Conversions|ToTransform(Vector) (Variables|Default|GetCurrentTargetLocation)) "AdjustIfPossibleButDontSpawnIfColliding" 0 0))
            (bind _output_get (Variables|Default|SetBP_LuccaChair _returnvalue))
            (bind _returnvalue_2 (Utilities|Array|Add (Variables|Default|GetBP_LuccaChairArray) _output_get))
            (Variables|Default|SetCurrentMeshIndex _returnvalue_2))
          (:BetterChair
            (bind _returnvalue_3 (Game|SpawnActorfromClass 0 (Math|Conversions|ToTransform(Vector) (Variables|Default|GetCurrentTargetLocation)) "AdjustIfPossibleButDontSpawnIfColliding" 0 0))
            (bind _output_get_2 (Variables|Default|SetBP_TeatroChair _returnvalue_3))
            (bind _returnvalue_4 (Utilities|Array|Add (Variables|Default|GetBP_TeatroChairArray) _output_get_2))
            (Variables|Default|SetCurrentMeshIndex _returnvalue_4)))
        (Variables|Default|SetCurrentChairsInRow (+ (Variables|Default|GetCurrentChairsInRow) 1))
        (Variables|Default|SetIndex2ndLoop_Targets (+ (Variables|Default|GetIndex2ndLoop_Targets) 1))
        (if (> (Variables|Default|GetIndex2ndLoop_Targets) (Variables|Default|GetChairsInRow))
          (Variables|Default|SetIndex2ndLoop_Targets 0))
        (for _index_2 (range (Variables|Default|GetIndex2ndLoop_Targets) (Variables|Default|GetIndex2ndLoop_Targets))
          (Variables|Default|SetCurrentTargetIndexx _index_2)
          (if (>= (Variables|Default|GetCurrentChairsInRow) (Variables|Default|GetChairsInRow))
            (Variables|Default|SetCurrentChairsInRow -1)
            (Variables|Default|SetRowLocation (+ (Variables|Default|GetRowLocation) "0,150.000000, 0")))
          (Variables|Default|SetCurrentTargetLocation (- (Transformation|GetActorLocation (Utilities|Array|Get(acopy) (Variables|Default|GetTargets) (Variables|Default|GetCurrentTargetIndexx))) (Variables|Default|GetRowLocation)))
          (Rendering|SetActorHiddenInGame false)
          (Transformation|SetActorLocationAndRotation (Utilities|Array|Get(acopy) (Variables|Default|GetBP_BasicChairsArray) (Variables|Default|GetCurrentMeshIndex)) (- (Transformation|GetActorLocation (Utilities|Array|Get(acopy) (Variables|Default|GetTargets) (Variables|Default|GetCurrentTargetIndexx))) (Variables|Default|GetRowLocation)) (Transformation|GetActorRotation (Utilities|Array|Get(acopy) (Variables|Default|GetTargets) (Variables|Default|GetCurrentTargetIndexx))))))
      (Variables|Default|SetRowLocation "0, 0, 0")
      (Variables|Default|SetCurrentTargetLocation "0, 0, 0")
      (Variables|Default|SetCurrentChairsInRow 0)
      (Variables|Default|SetIndex2ndLoop_Targets 0))))

(fn ConstructionScript)