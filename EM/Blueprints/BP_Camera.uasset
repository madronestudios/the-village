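; BP_Camera is a player-controlled camera Blueprint with movement, look and externally set placement.
; ChangeCamera snaps to a supplied world location and rotation without sweeping.
; MoveForward offsets the Camera component along world X by MoveSpeed without frame-time scaling, while MoveRight feeds movement input along the actor's right vector.
; TurnRate and LookUpRate drive controller yaw and pitch, scaled by base rates and delta time.
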(event Custom|ChangeCamera
  (params (Vect :type Vector :default "0, 0, 0") (rot :type Rotator :default "0, 0, 0"))
  (Transformation|SetWorldLocationAndRotation self Vect rot false))

(event Input|AxisEvents|InputAxisMoveForward
  (params (AxisValue :type Float%20%28single-precision%29))
  (Transformation|AddWorldOffset (Variables|Default|GetCamera) (Math|Vector|MakeVector (* AxisValue (Variables|Default|GetMoveSpeed)) 0.0 0.0) false))

(event Input|AxisEvents|InputAxisMoveRight
  (params (AxisValue :type Float%20%28single-precision%29))
  (Pawn|Input|AddMovementInput (Transformation|GetActorRightVector) AxisValue false))

(event Input|AxisEvents|InputAxisTurnRate
  (params (AxisValue :type Float%20%28single-precision%29))
  (Pawn|Input|AddControllerYawInput (* AxisValue (Variables|Default|GetBaseTurnRate) (Utilities|Time|GetWorldDeltaSeconds))))

(event Input|AxisEvents|InputAxisLookUpRate
  (params (AxisValue :type Float%20%28single-precision%29))
  (Pawn|Input|AddControllerPitchInput (* AxisValue (Variables|Default|GetBaseLookUpRate) (Utilities|Time|GetWorldDeltaSeconds))))

(fn ConstructionScript)