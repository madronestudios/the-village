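; BP_zkPoints is a Blueprint that spawns a row of chairs from a reference point actor.
; SpawnChairs loops over the chair count, spawning at CurrentPoint, storing each actor in ChairArray, then offsetting it by a growing vector with a fixed rotation.
; The Points event sets Point, but the branch that would pick CurrentPoint from several points by index is disconnected, and the spawn node has no class set.
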(event Custom|Points
  (params (NewParam :type Actor%20Object%20Reference))
  (Variables|Default|Setpoint NewParam))

(event Custom|SpawnChairs
  (for _index (range 0 (Variables|Default|GetNumberOfChairs))
    (bind _returnvalue (Game|SpawnActorfromClass 0 (Math|Conversions|ToTransform(Vector) (Transformation|GetActorLocation (Variables|Default|GetCurrentPoint))) "AdjustIfPossibleButDontSpawnIfColliding" 0 0))
    (bind _output_get (Variables|Default|SetCurrentChair _returnvalue))
    (bind _returnvalue_2 (Utilities|Array|Add (Variables|Default|GetChairArray) _output_get))
    (Variables|Default|SetCurrentIndex _returnvalue_2)
    ;[1 1 1] Comment
    (Transformation|SetActorLocationAndRotation (Variables|Default|GetCurrentChair) (+ (Transformation|GetActorLocation (Variables|Default|GetCurrentPoint)) (Variables|Default|GetPlusVector)) "0.000000,45.000000, 0")
    (Variables|Default|SetPlusVector (+ (Variables|Default|GetPlusVector) "80.000000,40.000000, 0"))))

(fn ConstructionScript)