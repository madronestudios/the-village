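; BP_LightsSetups manages the visibility of a set of point lights, either hiding all of them or applying an on/off pattern.
; It stores the supplied light array and forwards it to BP_Moods.
; LightsTurnOff stores a boolean array, waits briefly, then loops over the lights to set visibility.
; True means visible despite the LightsToTurnOff name, and a separate wrapping counter reads flags one index ahead of each light.
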(event Custom|LightsTurnOff
  (params (Array :type Array%20of%20Booleans))
  ;[1 1 1] Set arrays
  (Variables|Default|SetLightsToTurnOff Array)
  (Utilities|FlowControl|Delay 0.1)
  (CallFunction|ArrayLoopforLightsVisibility))

(event Custom|ResetLights
  ;[1 1 1] Turn off all lights
  (for (_ _array_index) (Variables|Default|GetLightsArray)
    (bind _aspoint_light (Utilities|Casting|CastToPointLight (Utilities|Array|Get(acopy) (Variables|Default|GetLightsArray) _array_index)))
    (bind _output_get (Variables|Default|SetCurrentLight _aspoint_light))
    (Rendering|SetVisibility _output_get false false)))

(event Custom|SetBPMoods
  (params (BP_moods :type BP%20Moods%20Object%20Reference))
  ;[1 1 1] Communication with BP_Moods
  (Variables|Default|SetBP_Moods BP_moods))

(event Custom|SetLightsArray
  (params (Lights :type Array%20of%20Actor%20Object%20References))
  ;[1 1 1] Set arrays
  (Variables|Default|SetLightsArray Lights)
  ;[1 1 1] Communication with BP_Moods
  (bind _asbp_moods (Utilities|Casting|CastToBP_Moods (Variables|Default|GetBP_Moods)))
  (Default|LightsArr _asbp_moods (Variables|Default|GetLightsArray)))

(event Custom|ArrayLoopForLightsVisibility
  (bind _lightsarray (Variables|Default|GetLightsArray))
  (bind _returnvalue (Utilities|Array|Length _lightsarray))
  ;[1 1 1] Loop bool visibility lights
  (for _index (range 0 _returnvalue)
    (Variables|Default|SetCurrentIndex _index)
    (Variables|Default|SetCurrentBoolIndex (+ 1 (Variables|Default|GetCurrentBoolIndex)))
    (if (> (Variables|Default|GetCurrentBoolIndex) _returnvalue)
      (Variables|Default|SetCurrentBoolIndex 0))
    (if (Utilities|Array|Get(acopy) (Variables|Default|GetLightsToTurnOff) (Variables|Default|GetCurrentBoolIndex))
      (bind _aspoint_light (Utilities|Casting|CastToPointLight (Utilities|Array|Get(acopy) (Variables|Default|GetLightsArray) (Variables|Default|GetCurrentIndex))))
      (bind _output_get (Variables|Default|SetCurrentLight _aspoint_light))
      (Rendering|SetVisibility _output_get true false)
      (else
        (bind _aspoint_light_2 (Utilities|Casting|CastToPointLight (Utilities|Array|Get(acopy) (Variables|Default|GetLightsArray) (Variables|Default|GetCurrentIndex))))
        (bind _output_get_2 (Variables|Default|SetCurrentLight _aspoint_light_2))
        (Rendering|SetVisibility _output_get_2 false false))))
  (Variables|Default|SetCurrentBoolIndex 0))

(fn ConstructionScript)