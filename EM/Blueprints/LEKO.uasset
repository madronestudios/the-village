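; LEKO is a placeable stage spotlight fixture that aims itself at an editable end point, LEKOEND.
; Its construction script applies intensity, color and cone angles to the spotlight, with attenuation radius either set directly or derived from the end point's distance.
; The holder takes only the look-at yaw and the light body only the pitch, splitting the aim like a real pan-and-tilt mount.
; A dynamic material instance makes the bulb match the light color, brightened.
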(event EventBeginPlay)

(event Collision|EventActorBeginOverlap
  (params (OtherActor :type Actor%20Object%20Reference)))

(event EventTick
  (params (DeltaSeconds :type Float%20%28single-precision%29)))

(fn ConstructionScript
  (bind _spotlight (Variables|Default|GetSpotLight))
  (bind _color (Variables|Default|GetColor))
  (Rendering|Components|Light|SetIntensity _spotlight (Variables|Default|GetIntensity))
  (Rendering|Components|Light|SetLightColor _spotlight _color true)
  (Variables|Default|SetBulbColor _color)
  (if (Variables|Default|GetUse%20End%20Point%20Distance)
    (Rendering|Lighting|SetAttenuationRadius (Variables|Default|GetSpotLight) (+ (Math|Vector|VectorLength (Variables|Default|GetLEKO%20END)) 7e+02))
    (else
      (Rendering|Lighting|SetAttenuationRadius _spotlight (Variables|Default|GetAttenuation%20Radius))))
  (Rendering|Lighting|SetInnerConeAngle _spotlight (Variables|Default|GetInner%20Cone%20Angle))
  (Rendering|Lighting|SetOuterConeAngle _spotlight (Variables|Default|GetOuter%20Cone%20Angle))
  (Transformation|SetRelativeRotation (Variables|Default|GetLECCO_holder) (Math|Rotator|MakeRotator 0.0 0.0 (.Yaw (Math|Rotator|BreakRotator (Math|Rotator|FindLookatRotation (Variables|/Script/Engine.SceneComponent|GetRelativeLocation (Variables|Default|GetLECCO_holder)) (Variables|Default|GetLEKO%20END))))) false false)
  (Transformation|SetRelativeRotation (Variables|Default|GetLECCO_light) (Math|Rotator|MakeRotator 0.0 (.Pitch (Math|Rotator|BreakRotator (Math|Rotator|FindLookatRotation (Variables|/Script/Engine.SceneComponent|GetRelativeLocation (Variables|Default|GetLECCO_light)) (+ (Variables|Default|GetLEKO%20END) "0, 0,50.000000")))) 0.0) false false)
  (bind _returnvalue (Rendering|Material|CreateDynamicMaterialInstance 0 0 :!class /Script/Engine.PrimitiveComponent))
  (Rendering|Material|SetVectorParameterValue _returnvalue "BulbColor" (* (Variables|Default|GetBulbColor) 1e+01) :!class /Script/Engine.MaterialInstanceDynamic))