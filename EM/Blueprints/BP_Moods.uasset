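; BP_Moods sets lighting moods by recoloring point lights from an array passed in through the LightsArr event.
; PinkPattern and BluePattern treat their pattern arrays as light indices, coloring only the first three and four entries respectively.
; FlipFlopPattern loops over all lights through a FlipFlop, alternating LightColor02 and a hardcoded yellow from one light to the next.
; A disconnected FlipFlop branch for the first light never runs.
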(event Custom|LightsArr
  (params (arr :type Array%20of%20Actor%20Object%20References))
  (Variables|Default|SetLightsArray arr))

(event Custom|PinkPattern
  (for (_array_element _array_index) (Variables|Default|GetMoodPattern_Pink)
    (Variables|Default|SetCurrentPinkPattern _array_element)
    (if (not (>= _array_index 3))
      (bind _aspoint_light (Utilities|Casting|CastToPointLight (Utilities|Array|Get(acopy) (Variables|Default|GetLightsArray) (Variables|Default|GetCurrentPinkPattern))))
      (Rendering|Components|Light|SetLightColor _aspoint_light (Variables|Default|GetLightColor)))))

(event Custom|BluePattern
  (for (_array_element _array_index) (Variables|Default|GetMoodPattern_Blue)
    (Variables|Default|SetCurrentBluePattern _array_element)
    (if (not (>= _array_index 4))
      (bind _aspoint_light (Utilities|Casting|CastToPointLight (Utilities|Array|Get(acopy) (Variables|Default|GetLightsArray) (Variables|Default|GetCurrentBluePattern))))
      (Rendering|Components|Light|SetLightColor _aspoint_light (Variables|Default|GetLightColor02)))))

(event Custom|FlipFlopPattern
  (for (_ _array_index) (Variables|Default|GetLightsArray)
    (Utilities|FlowControl|FlipFlop
      (:A
        (bind _aspoint_light (Utilities|Casting|CastToPointLight (Utilities|Array|Get(acopy) (Variables|Default|GetLightsArray) _array_index)))
        (Rendering|Components|Light|SetLightColor _aspoint_light (Variables|Default|GetLightColor02)))
      (:B
        (bind _aspoint_light_2 (Utilities|Casting|CastToPointLight (Utilities|Array|Get(acopy) (Variables|Default|GetLightsArray) _array_index)))
        (Rendering|Components|Light|SetLightColor _aspoint_light_2 "(R=0.795000,G=0.713577,B=0.107325,A=1.000000)")))))

(fn ConstructionScript)