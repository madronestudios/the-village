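; BP_FurnitureSetups positions an array of furniture mesh actors at the locations of target actors.
; Setter events receive both arrays, and setting the targets (noted as coming from UI) triggers the placement loop.
; The loop moves each mesh without sweep to a target chosen by a persistent counter, which increments per mesh and resets to zero after exceeding the mesh count.
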(event Custom|ArrayLoopForLocation
  (bind _meshes (Variables|Default|GetMeshes))
  (bind _returnvalue (Utilities|Array|Length _meshes))
  ;[1 1 1] Set locations
  ;  to meshes
  (for _index (range 0 _returnvalue)
    (Variables|Default|SetCurrentMeshIndex _index)
    (Variables|Default|SetIndex2ndLoop_Targets (+ (Variables|Default|GetIndex2ndLoop_Targets) 1))
    (if (> (Variables|Default|GetIndex2ndLoop_Targets) _returnvalue)
      (Variables|Default|SetIndex2ndLoop_Targets 0))
    (for _index_2 (range (Variables|Default|GetIndex2ndLoop_Targets) (Variables|Default|GetIndex2ndLoop_Targets))
      (Variables|Default|SetCurrentTargetIndexx _index_2)
      (bind _output_get (Variables|Default|SetCurrentTargetLocation (Transformation|GetActorLocation (Utilities|Array|Get(acopy) (Variables|Default|GetTargets) (Variables|Default|GetCurrentTargetIndexx)))))
      (Transformation|SetActorLocation (Utilities|Array|Get(acopy) (Variables|Default|GetMeshes) (Variables|Default|GetCurrentMeshIndex)) _output_get false))))

(event Custom|SetTargetsArray
  (params (Targets :type Array%20of%20Actor%20Object%20References))
  ;[1 1 1] Set targets array from UI
  (Variables|Default|SetTargets Targets)
  (CallFunction|ArrayLoopforLocation))

(event Custom|SetFurnitureMeshArray
  (params (Meshes :type Array%20of%20Actor%20Object%20References))
  ;[1 1 1] Set furniture meshes
  (Variables|Default|SetMeshes Meshes))

(fn ConstructionScript)